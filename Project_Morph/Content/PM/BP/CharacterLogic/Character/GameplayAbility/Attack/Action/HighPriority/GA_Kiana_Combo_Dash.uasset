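; Gameplay ability for Kiana's combo dash, playing a front or back evade montage and ending when it finishes or is interrupted.
; On activation, the angle between last input and actor forward, tested against half of FaceZoneAngle, picks the direction.
; MotionWarp sets a "Dash" warp target WarpingDistance along current acceleration, or actor forward if none.
; Back dashes with input reverse the target rotation to face away from travel.
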(event `self.K2_ActivateAbility`
  (bind _output_get (set `self.bIsDashFront` (< (`KismetMathLibrary.RadiansToDegrees` (`KismetMathLibrary.Acos` (`KismetMathLibrary.Dot_VectorVector` (`PawnMovementComponent.GetLastInputVector` (`Character.CharacterMovement` (`self.GetHeroCharacterFromActorInfo`))) (`Actor.GetActorForwardVector` (`self.GetHeroCharacterFromActorInfo`))))) (/ (`self.FaceZoneAngle`) 2.0))))
  (if _output_get
    (set `self.Montage to Play` "/Game/KianaResources/MontageRootBone/AM_Kiana_Evade_Front.AM_Kiana_Evade_Front")
    (else
      (set `self.Montage to Play` "/Game/KianaResources/MontageRootBone/AM_Kiana_Evade_Back.AM_Kiana_Evade_Back")))
  (`parent.K2_ActivateAbility`))

(event `self.EventPlayMontage`
  (if (`self.bIsDashFront`)
    (`AbilityTask_PlayMontageAndWait.CreatePlayMontageAndWaitProxy` "None" (`self.Montage to Play`)
      (:`OnCompleted`
        _)
      (:`OnBlendOut`
        _)
      (:`OnInterrupted`
        _)
      (:`OnCancelled`
        _))
    (`self.K2_EndAbility`)
    (else
      (`AbilityTask_PlayMontageAndWait.CreatePlayMontageAndWaitProxy` "None" (`self.Montage to Play`)
        (:`OnCompleted`
          _)
        (:`OnBlendOut`
          _)
        (:`OnInterrupted`
          _)
        (:`OnCancelled`
          _))
      (`self.K2_EndAbility`))))

(event `self.K2_OnEndAbility`
  (params (bWasCancelled :type Boolean))
  (`parent.K2_OnEndAbility` bWasCancelled))

(fn `MotionWarp`
  (locals (CurrentInputVector :type "Vector Structure" :default (0.0 0.0 0.0)) (CurrentPlayerVector :type "Vector Structure" :default (0.0 0.0 0.0)))
  (bind _returnvalue (`Actor.GetActorForwardVector` (`self.GetHeroCharacterFromActorInfo`)))
  (`MotionWarpingComponent.RemoveWarpTarget` (`Actor.GetComponentByClass` (`self.GetHeroCharacterFromActorInfo`) "/Script/MotionWarping.MotionWarpingComponent") "Dash")
  (bind _output_get (set `local.CurrentInputVector` (`KismetMathLibrary.Normal` (`CharacterMovementComponent.GetCurrentAcceleration` (`Character.CharacterMovement` (`self.GetHeroCharacterFromActorInfo`))))))
  (set `local.CurrentPlayerVector` (`Actor.K2_GetActorLocation` (`self.GetHeroCharacterFromActorInfo`)))
  (if (!= _output_get (0.0 0.0 0.0) :`ErrorTolerance` 0.01)
    (`MotionWarpingComponent.AddOrUpdateWarpTargetFromLocationAndRotation` (`Actor.GetComponentByClass` (`self.GetHeroCharacterFromActorInfo`) "/Script/MotionWarping.MotionWarpingComponent") "Dash" (+ (* (`local.CurrentInputVector`) (`self.WarpingDistance`)) (`local.CurrentPlayerVector`)) (`KismetMathLibrary.Conv_VectorToRotator` (* (`local.CurrentInputVector`) (`KismetMathLibrary.SelectFloat` 1.0 -1.0 (`self.bIsDashFront`)))))
    (else
      (`MotionWarpingComponent.AddOrUpdateWarpTargetFromLocationAndRotation` (`Actor.GetComponentByClass` (`self.GetHeroCharacterFromActorInfo`) "/Script/MotionWarping.MotionWarpingComponent") "Dash" (+ (* _returnvalue (`self.WarpingDistance`)) (`local.CurrentPlayerVector`)) (`KismetMathLibrary.Conv_VectorToRotator` _returnvalue)))))