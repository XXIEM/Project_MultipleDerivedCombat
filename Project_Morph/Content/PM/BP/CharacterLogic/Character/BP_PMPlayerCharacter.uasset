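; BP_PMPlayerCharacter is the player character Blueprint, handling lock-on camera aim and the hero attribute UI.
; While the ability system has the IsLockingEnemy tag, Tick interpolates control pitch and yaw toward the combat component's locked enemy, aiming below its location and preserving roll.
; BeginPlay creates the attribute widget with a reference to the character, adds it to the viewport, then initializes it after a short delay.
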(event `self.ReceiveTick`
  (params (DeltaSeconds :type "Float (single-precision)"))
  (bind _returnvalue (`self.GetController`))
  (bind _returnvalue_2 (`self.K2_GetActorRotation` _returnvalue))
  (bind (_returnvalue_x _returnvalue_y _returnvalue_z) (`KismetMathLibrary.BreakVector` (`self.K2_GetActorLocation` (`HeroCombatComponent.GetCurrentLockedEnemy` (`self.HeroCombatComponent`)))))
  (bind (_returnvalue_roll _returnvalue_pitch _returnvalue_yaw) (`KismetMathLibrary.BreakRotator` (`KismetMathLibrary.RInterpTo` _returnvalue_2 (`KismetMathLibrary.FindLookAtRotation` (`self.K2_GetActorLocation`) (`KismetMathLibrary.MakeVector` _returnvalue_x _returnvalue_y (+ _returnvalue_z -80.0))) (`GameplayStatics.GetWorldDeltaSeconds`) 5.0)))
  (if (`GameplayTagAssetInterface.HasMatchingGameplayTag` (`self.PMAbilitySystemComponent`) (struct :`TagName` "PM.State.Action.IsLockingEnemy"))
    (`Controller.SetControlRotation` _returnvalue (`KismetMathLibrary.MakeRotator` (.roll _returnvalue_2) _returnvalue_pitch _returnvalue_yaw))))

(event `self.ReceiveBeginPlay`
  (bind _uw_attribute (`self.UW_Attribute`))
  (bind _returnvalue (`|CreateWidget` "/Game/PM/BP/UI/UW_HeroAttribute.UW_HeroAttribute_C" (`GameplayStatics.GetPlayerController` 0) self))
  (set `self.UW_Attribute` _returnvalue)
  (`parent.ReceiveBeginPlay`)
  (`UserWidget.AddToViewport` _uw_attribute 0)
  (`KismetSystemLibrary.Delay` 0.2)
  (`/Game/PM/BP/UI/UW_HeroAttribute.Init` _uw_attribute))

(fn `UserConstructionScript`)