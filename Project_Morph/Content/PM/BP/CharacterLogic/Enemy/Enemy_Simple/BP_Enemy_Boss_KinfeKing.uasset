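; Blueprint for the Knife King boss enemy, which puts its own attribute widget on screen when play begins.
; BeginPlay creates a UW_EnemyAttribute widget bound to this character and owned by player controller 0, then runs the parent logic.
; It adds the widget to the viewport and initializes it after a short delay.
; The construction script only calls the parent.
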(event `self.ReceiveBeginPlay`
  (bind _uw_attribute (`self.UW_Attribute`))
  (bind _returnvalue (`|CreateWidget` "/Game/PM/BP/UI/UW_EnemyAttribute.UW_EnemyAttribute_C" (`GameplayStatics.GetPlayerController` 0) self))
  (set `self.UW_Attribute` _returnvalue)
  (`parent.ReceiveBeginPlay`)
  (`UserWidget.AddToViewport` _uw_attribute 0)
  (`KismetSystemLibrary.Delay` 0.2)
  (`/Game/PM/BP/UI/UW_EnemyAttribute.Init` _uw_attribute))

(fn `UserConstructionScript`
  (`parent.UserConstructionScript`))