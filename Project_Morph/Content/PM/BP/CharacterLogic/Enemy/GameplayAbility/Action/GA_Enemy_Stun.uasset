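; Enemy gameplay ability that handles stun hit reactions, triggered by the stun action event.
; It spawns a Niagara hit effect at the impact, then, if the enemy has the CanStun tag, picks one of two KnifeKing montages by whether the event target is within the front angle.
; The ability ends right after starting the montage, whose finish or interruption callbacks send the next-combo event.
; Motion-warp logic is present but disconnected.
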(event `self.K2_ActivateAbilityFromEvent`
  (params (EventData :type "GameplayEventData Structure (by ref)"))
  (bind _returnvalue (`self.GetEnemyCharacterFromActorInfo`))
  (bind (_bblockinghit _binitialoverlap _time _distance _location _impactpoint _normal _impactnormal) (`GameplayStatics.BreakHitResult` (`AbilitySystemBlueprintLibrary.GetHitResultFromTargetData` (`.TargetData` (break `GameplayEventData` EventData)))))
  (if (`BlueprintGameplayTagLibrary.HasTag` (`BlueprintGameplayTagLibrary.MakeLiteralGameplayTagContainer` (struct :`GameplayTags` (struct :`(TagName` "PM.Event.Action.Stun")))) (`.EventTag` (break `GameplayEventData` EventData)))
    (`NiagaraFunctionLibrary.SpawnSystemAtLocation` "/Game/PM/VFX/Niagara/NS_HitEffect.NS_HitEffect" _impactpoint (`KismetMathLibrary.Conv_VectorToRotator` _impactnormal) (1.0 1.0 1.0) true true "AutoRelease")
    (if (`GameplayTagAssetInterface.HasMatchingGameplayTag` (`self.GetPMAbilitySystemComponentFromActorInfo`) (struct :`TagName` "PM.State.Action.CanStun"))
      (if (< (`KismetMathLibrary.RadiansToDegrees` (`KismetMathLibrary.Acos` (`KismetMathLibrary.Dot_VectorVector` (`KismetMathLibrary.Normal` (- (`Actor.K2_GetActorLocation` (`.Target` (break `GameplayEventData` EventData))) (`Actor.K2_GetActorLocation` _returnvalue))) (`Actor.GetActorForwardVector` _returnvalue)))) (/ (`self.FrontZoneAngle`) 2.0))
        (`|PlayMontage` (`self.GetOwningComponentFromActorInfo`) "/Game/StrikeJaegerResources/MontageRootBone/AM_KnifeKing_Hit_B_Long.AM_KnifeKing_Hit_B_Long"
          (:`then`
            _)
          (:`OnCompleted`
            (`self.SendGameplayEvent` (struct :`TagName` "PM.Enemy.Event.ActivateNextCombo") :!label _label))
          (:`OnBlendOut`
            (goto _label))
          (:`OnInterrupted`
            (goto _label)))
        (`self.K2_EndAbility`)
        (else
          (`|PlayMontage` (`self.GetOwningComponentFromActorInfo`) "/Game/StrikeJaegerResources/MontageRootBone/AM_KnifeKing_Hit_F_Short.AM_KnifeKing_Hit_F_Short"
            (:`then`
              _)
            (:`OnCompleted`
              (`self.SendGameplayEvent` (struct :`TagName` "PM.Enemy.Event.ActivateNextCombo") :!label _label_2))
            (:`OnBlendOut`
              (goto _label_2))
            (:`OnInterrupted`
              (goto _label_2)))
          (`self.K2_EndAbility`)))
      (else
        (`self.K2_EndAbility`)))
    (else
      (`self.K2_EndAbility`))))

(fn `MotionWarp`
  (params (Target :type "Actor Object Reference"))
  (returns (ReturnLoc :type "Vector Structure") (ReturnRot :type "Rotator Structure"))
  (bind _returnvalue (`self.GetEnemyCharacterFromActorInfo`))
  (bind _returnvalue_2 (`Actor.K2_GetActorLocation` _returnvalue))
  (return (+ (* (`Actor.GetActorForwardVector` _returnvalue) -200.0) _returnvalue_2) (`KismetMathLibrary.FindLookAtRotation` _returnvalue_2 (+ (`Actor.K2_GetActorLocation` Target) (* (`Actor.GetActorForwardVector` Target) -100.0)))))