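; Enemy combo attack gameplay ability variant for a retreating attack that turns the enemy toward its locked target.
; MotionWarp sets the RetreatAttack warp target a WarpingDistance behind the enemy, rotated to look at the combat component's locked enemy.
; GetDamageLoc returns the locked enemy's location plus its forward vector, with 50 added to that vector rather than scaling it.
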(fn `GetDamageLoc`
  (returns (ReturnValue :type "Vector Structure"))
  (bind _returnvalue (`PawnCombatComponent.GetCurrentLockedEnemy` (`self.GetEnemyCombatComponentFromActorInfo`)))
  (return (+ (`Actor.K2_GetActorLocation` _returnvalue) (+ (`Actor.GetActorForwardVector` _returnvalue) 50.0))))

(fn `MotionWarp`
  (bind _returnvalue (`Actor.K2_GetActorLocation` (`self.GetEnemyCharacterFromActorInfo`)))
  (`MotionWarpingComponent.AddOrUpdateWarpTargetFromLocationAndRotation` (`Actor.GetComponentByClass` (`self.GetEnemyCharacterFromActorInfo`) "/Script/MotionWarping.MotionWarpingComponent") "RetreatAttack" (+ (* (* (`Actor.GetActorForwardVector` (`self.GetEnemyCharacterFromActorInfo`)) -1.0) (`self.WarpingDistance`)) _returnvalue) (`KismetMathLibrary.FindLookAtRotation` _returnvalue (`Actor.K2_GetActorLocation` (`PawnCombatComponent.GetCurrentLockedEnemy` (`self.GetEnemyCombatComponentFromActorInfo`))))))