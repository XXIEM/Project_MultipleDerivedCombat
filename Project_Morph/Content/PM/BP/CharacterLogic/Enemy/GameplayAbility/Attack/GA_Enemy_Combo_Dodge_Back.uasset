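; Enemy gameplay ability for a backward dodge, named as part of a combo, that sets up motion warping for the dash.
; Its MotionWarp function updates the "Dash" warp target to a fixed distance directly behind the enemy character.
; The target rotation faces the currently locked enemy taken from the combat component, so the character retreats while looking at its opponent.
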(fn `MotionWarp`
  (bind _returnvalue (`Actor.K2_GetActorLocation` (`self.GetEnemyCharacterFromActorInfo`)))
  (`MotionWarpingComponent.AddOrUpdateWarpTargetFromLocationAndRotation` (`Actor.GetComponentByClass` (`self.GetEnemyCharacterFromActorInfo`) "/Script/MotionWarping.MotionWarpingComponent") "Dash" (+ (* (* (`Actor.GetActorForwardVector` (`self.GetEnemyCharacterFromActorInfo`)) -1.0) 500.0) _returnvalue) (`KismetMathLibrary.FindLookAtRotation` _returnvalue (`Actor.K2_GetActorLocation` (`PawnCombatComponent.GetCurrentLockedEnemy` (`self.GetEnemyCombatComponentFromActorInfo`))))))