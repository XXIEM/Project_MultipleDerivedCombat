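; BP_AnimTestCharacter is a player-controlled test character for animation, using Enhanced Input and a linked animation layer.
; BeginPlay adds the default mapping context to player 0's input subsystem and links ABP_BasicLocomotionLayer to the mesh's anim instance.
; The move action drives movement relative to control yaw with pitch zeroed, and the look action feeds controller yaw and pitch.
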(event `self.ReceiveBeginPlay`
  (`EnhancedInputSubsystemInterface.AddMappingContext` (pcsubsystem `EnhancedInputLocalPlayerSubsystem` (`GameplayStatics.GetPlayerController` 0)) "/Game/PM/BP/CharacterLogic/Character/Input/IMC_Default.IMC_Default" 0 (struct))
  (`SkeletalMeshComponent.LinkAnimClassLayers` (`self.Mesh`) "/Game/Test/AnimTest/ABP_BasicLocomotionLayer.ABP_BasicLocomotionLayer_C"))

(event `EnhancedInput|/Game/PM/BP/CharacterLogic/Character/Input/Actions/IA_Move`
  (params (ActionValue :type "Vector2D Structure") (ElapsedSeconds :type "Float (double-precision)") (TriggeredSeconds :type "Float (double-precision)") (InputAction :type "InputAction Object Reference" :default "/Game/PM/BP/CharacterLogic/Character/Input/Actions/IA_Move.IA_Move"))
  (bind (_returnvalue_roll _returnvalue_pitch _returnvalue_yaw) (`KismetMathLibrary.BreakRotator` (`self.GetControlRotation`)))
  (bind (_x _y) (`KismetMathLibrary.BreakVector2D` ActionValue))
  (:`Triggered`
    (`self.AddMovementInput` (`KismetMathLibrary.GetForwardVector` (`KismetMathLibrary.MakeRotator` _returnvalue_roll 0.0 _returnvalue_yaw)) _y)
    (`self.AddMovementInput` (`KismetMathLibrary.GetRightVector` (`KismetMathLibrary.MakeRotator` 0.0 0.0 _returnvalue_yaw)) _x)))

(event `EnhancedInput|/Game/PM/BP/CharacterLogic/Character/Input/Actions/IA_Look`
  (params (ActionValue :type "Vector2D Structure") (ElapsedSeconds :type "Float (double-precision)") (TriggeredSeconds :type "Float (double-precision)") (InputAction :type "InputAction Object Reference" :default "/Game/PM/BP/CharacterLogic/Character/Input/Actions/IA_Look.IA_Look"))
  (bind (_x _y) (`KismetMathLibrary.BreakVector2D` ActionValue))
  (:`Triggered`
    (`self.AddControllerYawInput` _x)
    (`self.AddControllerPitchInput` _y)))

(fn `UserConstructionScript`)